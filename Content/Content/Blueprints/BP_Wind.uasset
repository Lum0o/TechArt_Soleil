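; BP_Wind is a wind actor that turns particle data exported from its Niagara effect into physical hitbox actors.
; On BeginPlay it registers itself as the Niagara callback object to receive particle data.
; For each particle received, it spawns a BP_WindHitbox at that position with the wind actor's rotation and scale.
; The particle's Size field sets the hitbox lifespan, and its velocity drives the hitbox sphere's physics velocity.
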(event EventBeginPlay
  (Niagara|SetNiagaraVariable(Object) (Variables|Default|GetNiagara) "User.BPCallback" self))

(event EventParticleData
  (params (Data :type Array%20of%20Basic%20Particle%20Data%20Structures) (NiagaraSystem :type Niagara%20System%20Object%20Reference) (SimulationPositionOffset :type Vector%20%28by%20ref%29 :default "0, 0, 0"))
  (for _array_element Data
    (bind _returnvalue (Game|SpawnActorfromClass "/Game/Content/Blueprints/BP_WindHitbox.BP_WindHitbox_C" (Math|Transform|MakeTransform (.Position (Utilities|Struct|BreakBasicParticleData _array_element)) (Transformation|GetActorRotation) (Transformation|GetActorScale3D)) "AlwaysSpawn" "MultiplyWithRoot" 0 0))
    (Actor|SetLifeSpan _returnvalue (.Size (Utilities|Struct|BreakBasicParticleData _array_element)))
    (Class|PrimitiveComponent|SetAllPhysicsLinearVelocity (Variables|/Game/Content/Blueprints/BP_WindHitbox.BP_WindHitbox_C|GetSphere _returnvalue) (.Velocity (Utilities|Struct|BreakBasicParticleData _array_element)) false)))

(fn ConstructionScript)